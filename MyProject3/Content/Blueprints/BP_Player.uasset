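; BP_Player is the player in an obstacle-dodging runner, a physics cube pushed forward and steered sideways.
; BeginPlay adds the input mapping, starts a looping impulse timer, creates the HUD and passes it to BP_ScoreSystem to start the run.
; Enhanced Input adds sideways impulses while CanMove is true.
; Hitting an "Obstacle" actor disables steering and clears MoveTimerHandle, though this graph never assigns that handle.
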(event `EnhancedInput|/Game/Input/LeftRightMove`
  (params (ActionValue :type "Float (double-precision)") (ElapsedSeconds :type "Float (double-precision)") (TriggeredSeconds :type "Float (double-precision)") (InputAction :type "InputAction Object Reference" :default "/Game/Input/LeftRightMove.LeftRightMove"))
  (:`Triggered`
    (`KismetSystemLibrary.PrintString` (`KismetStringLibrary.Conv_DoubleToString` ActionValue))))

(event `self.ReceiveBeginPlay`
  (`KismetSystemLibrary.PrintString` "Hello World")
  (`|ExecutionSequence`
    (:`then_0`
      (bind _asplayer_controller (cast `PlayerController` (`self.GetController`)))
      (`EnhancedInputSubsystemInterface.AddMappingContext` (pcsubsystem `EnhancedInputLocalPlayerSubsystem` _asplayer_controller) "/Game/Input/PlayerInput.PlayerInput" 0 (struct)))
    (:`then_1`
      (`KismetSystemLibrary.K2_SetTimerDelegate` (delegate `CubeMove`) 0.1 true))
    (:`then_2`
      (bind _returnvalue (`|CreateWidget` "/Game/UI/WP_PlayerUI.WP_PlayerUI_C"))
      (`UserWidget.AddToViewport` _returnvalue 0)
      (set `self.PlayerHUD` _returnvalue))
    (:`then_3`
      (bind _returnvalue_2 (`GameplayStatics.GetActorOfClass` "/Game/Blueprints/BP_ScoreSystem.BP_ScoreSystem_C"))
      (`/Engine/EditorBlueprintResources/StandardMacros.IsValid` _returnvalue_2
        (:`Is Valid`
          (bind _output_get (set `self.scoreSystem` _returnvalue_2))
          (`/Game/Blueprints/BP_ScoreSystem.OnRunStarted` _output_get (`self.PlayerHUD`)))))))

(event `CubeMove`
  (`PrimitiveComponent.AddImpulse` (`self.Cube`) (`KismetMathLibrary.MakeVector` (`self.CubeSpeed`)) "None" true))

(event `self.Cube.OnComponentHit`
  (params (HitComponent :type "PrimitiveComponent Object Reference") (OtherActor :type "Actor Object Reference") (OtherComp :type "PrimitiveComponent Object Reference") (NormalImpulse :type "Vector Structure") (Hit :type "HitResult Structure (by ref)"))
  ; Cube hit
  (if (`self.ActorHasTag` OtherActor "Obstacle")
    (set `self.CanMove` false)
    (`KismetSystemLibrary.PrintString` "GAME OVER!")
    (`KismetSystemLibrary.K2_ClearAndInvalidateTimerHandle` (`self.MoveTimerHandle`))))

(event `EnhancedInput|/Game/Input/LeftRightMove`
  (params (ActionValue :type "Float (double-precision)") (ElapsedSeconds :type "Float (double-precision)") (TriggeredSeconds :type "Float (double-precision)") (InputAction :type "InputAction Object Reference" :default "/Game/Input/LeftRightMove.LeftRightMove"))
  ; Movement LeftRight
  (:`Triggered`
    (if (`self.CanMove`)
      (`PrimitiveComponent.AddImpulse` (`self.Cube`) (`KismetMathLibrary.MakeVector` 0.0 (* ActionValue 10.0)) "None" true))))

(fn `UserConstructionScript`)