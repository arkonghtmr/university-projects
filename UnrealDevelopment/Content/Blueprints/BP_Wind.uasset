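; BP_Wind generates intermittent random wind gusts, exposed as state variables.
; From BeginPlay it waits a random delay, then StartWind sets the active flag and randomizes direction, duration and strength.
; When the duration ends it clears the flag and loops back to the delay, repeating indefinitely without Tick.
; The direction is a random 3D unit vector, and the Blueprint itself applies no force.
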(event `self.ReceiveBeginPlay`
  (`KismetSystemLibrary.Delay` (`KismetMathLibrary.RandomFloatInRange` 10.0 30.0) :!label _label)
  (`self.StartWind`))

(event `StartWind`
  (set `self.IsWindActive` true)
  (set `self.WindDirection` (`KismetMathLibrary.RandomUnitVector`))
  (set `self.WindDuration` (`KismetMathLibrary.RandomFloatInRange` 10.0 30.0))
  (set `self.WindStrenght` (`KismetMathLibrary.RandomFloatInRange` 500.0 1500.0))
  (`KismetSystemLibrary.Delay` (`self.WindDuration`))
  (set `self.IsWindActive` false)
  (goto _label))

(fn `UserConstructionScript`)